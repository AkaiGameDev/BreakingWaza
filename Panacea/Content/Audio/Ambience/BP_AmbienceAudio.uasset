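; Ambience audio Blueprint that starts wind, rain/cricket and music MetaSound sources when play begins.
; Events fade the wind and rain/cricket layers in or out together, leaving music playing.
; A separate event sets the music's DistortionAmount float parameter.
; Debug keys J, K and L print a message and drive that distortion at off, half and full strength.
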(event Custom|MusicDistortionAmount_Event
  (params (DistortionAmount :type Float%20%28double-precision%29))
  (Audio|Parameter|SetFloatParameter (Variables|Default|GetMSS_Music) "DistortionAmount" DistortionAmount :!class /Script/Engine.AudioComponent))

(event Custom|StopAmbienceSounds_Event
  (bind _fadeoutduration (Variables|Default|GetFadeoutDuration))
  (Audio|Components|Audio|FadeOut (Variables|Default|GetMSS_Rain_Cricket) _fadeoutduration 0.0 "Linear" :!class /Script/Engine.AudioComponent)
  (Audio|Components|Audio|FadeOut (Variables|Default|GetMSS_Wind) _fadeoutduration 0.0 "Linear" :!class /Script/Engine.AudioComponent))

(event Custom|StartAmbienceSounds_Event
  (bind _fadeinduration (Variables|Default|GetFadeinDuration))
  (Audio|Components|Audio|FadeIn (Variables|Default|GetMSS_Rain_Cricket) _fadeinduration 1.0 0.0 "Linear" :!class /Script/Engine.AudioComponent)
  (Audio|Components|Audio|FadeIn (Variables|Default|GetMSS_Wind) _fadeinduration 1.0 0.0 "Linear" :!class /Script/Engine.AudioComponent))

(event EventBeginPlay
  (Audio|Components|Audio|Play (Variables|Default|GetMSS_Wind) 0.0)
  (Audio|Components|Audio|Play (Variables|Default|GetMSS_Rain_Cricket) 0.0)
  (Audio|Components|Audio|Play (Variables|Default|GetMSS_Music) 0.0))

(event Input|KeyboardEvents|DebugKeyJ
  (params (Key :type Key%20Structure :default "None") (ActionValue :type Input%20Action%20Value%20Structure))
  (:Pressed
    (Development|PrintString "MuiscDistortionAmount: 0")
    (CallFunction|MusicDistortionAmountEvent 0.0)))

(event Input|KeyboardEvents|DebugKeyK
  (params (Key :type Key%20Structure :default "None") (ActionValue :type Input%20Action%20Value%20Structure))
  (:Pressed
    (Development|PrintString "MuiscDistortionAmount: 0.5")
    (CallFunction|MusicDistortionAmountEvent 0.5)))

(event Input|KeyboardEvents|DebugKeyL
  (params (Key :type Key%20Structure :default "None") (ActionValue :type Input%20Action%20Value%20Structure))
  (:Pressed
    (Development|PrintString "MuiscDistortionAmount: 1")
    (CallFunction|MusicDistortionAmountEvent 1.0)))

(fn ConstructionScript)