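; Trigger actor that plays a camera zoom toward a tagged target when the first-person character overlaps it.
; It is armed when the game mode's item-interacted event matches TriggerActor.
; On overlap, it locks game input, blends to a spawned camera facing the target, and narrows FOV through a timeline.
; It then blends back, restores input, disarms, and broadcasts its display name as an interacted item, allowing chained events.
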(event `self.ReceiveBeginPlay`
  (bind _asbp_panacea_game_mode (cast `/Game/Blueprints/BP_PanaceaGameMode` (`GameplayStatics.GetGameMode`)))
  (add `PanaceaGameMode.OnItemInteractedDelegate` _asbp_panacea_game_mode (delegate `CheckInteractable`)))

(event `CheckInteractable`
  (params (ItemName :type String))
  (if (== ItemName (`self.TriggerActor`))
    (set `self.bIsActive` true)))

(event `self.ReceiveActorBeginOverlap`
  (params (OtherActor :type "Actor Object Reference"))
  (bind _returnvalue (`GameplayStatics.GetPlayerController` 0))
  (bind _returnvalue_2 (`GameplayStatics.GetPlayerController` 0))
  (bind _out_blend_time (`self.Out Blend Time`))
  (bind _in_blend_time (`self.In Blend Time`))
  (bind _cameracomponent (`CameraActor.CameraComponent` (`self.CameraActor`)))
  (if (`self.bIsActive`)
    (bind _asbp_first_person_character (cast `/Game/Blueprints/BP_FirstPersonCharacter` OtherActor))
    (bind _output_get (set `self.First Person Character` _asbp_first_person_character))
    (set `self.CameraLocation` (`SceneComponent.K2_GetComponentToWorld` (`PanaceaCharacter.GetFirstPersonCameraComponent` _output_get)))
    (`WidgetBlueprintLibrary.SetInputMode_UIOnlyEx` _returnvalue null "DoNotLock" true)
    (bind _returnvalue_3 (`|SpawnActorFromClass` "/Script/Engine.CameraActor" (`self.CameraLocation`) "Undefined" "MultiplyWithRoot" null null))
    (bind _output_get_2 (set `self.CameraActor` _returnvalue_3))
    (`self.SetLookAtActorRotation`)
    (`PlayerController.SetViewTargetWithBlend` _returnvalue _output_get_2 _in_blend_time "VTBlend_EaseOut" 1.0 false)
    (`KismetSystemLibrary.Delay` _in_blend_time)
    (set `self.Original Field Of View` (`CameraComponent.FieldOfView` _cameracomponent))
    (bind (_direction _newtrack_0) (`Timeline|ZoomTimeline` :!via `PlayFromStart`)
      (:`Update`
        (`CameraComponent.SetFieldOfView` _cameracomponent (- (`self.Original Field Of View`) _newtrack_0)))
      (:`Finished`
        (`PlayerController.SetViewTargetWithBlend` _returnvalue_2 (`self.First Person Character`) _out_blend_time "VTBlend_Linear" 0.0 false)
        (`KismetSystemLibrary.Delay` _out_blend_time)
        (`WidgetBlueprintLibrary.SetInputMode_GameOnly` _returnvalue_2)
        (`self.K2_DestroyActor` (`self.CameraActor`))
        (set `self.bIsActive` false)
        (bind _asbp_panacea_game_mode (cast `/Game/Blueprints/BP_PanaceaGameMode` (`GameplayStatics.GetGameMode`)))
        (`PanaceaGameMode.BroadcastOnItemInteracted` _asbp_panacea_game_mode (`KismetSystemLibrary.GetDisplayName` self))))))

(fn `SetLookAtActorRotation`
  (bind _outactors (`GameplayStatics.GetAllActorsOfClassWithTag` (`self.Look At Actor`) (`self.ActorTag`)))
  (`self.K2_SetActorRotation` (`self.CameraActor`) (`KismetMathLibrary.FindLookAtRotation` (`self.K2_GetActorLocation` (`self.CameraActor`)) (`self.K2_GetActorLocation` (`|GetArrayItem` _outactors))) false))

(fn `UserConstructionScript`)