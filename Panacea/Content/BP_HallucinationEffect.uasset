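; Post-process actor that plays a hallucination and wavy-screen effect whenever an ingredient is added.
; On BeginPlay it creates dynamic instances of both materials, sets them as post-process blendables with zero intensity, and binds to the first-person GameMode's OnIngredientAdded event.
; Each event restarts a Timeline whose EffectIntensity track drives both materials' intensity parameters, regardless of the ingredient name.
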(event `self.ReceiveBeginPlay`
  (bind _returnvalue (`KismetMaterialLibrary.CreateDynamicMaterialInstance` "/Game/M_HallucinationFX.M_HallucinationFX"))
  (bind _output_get (set `self.HallucinationMaterialInstance` _returnvalue))
  (bind _returnvalue_2 (`KismetMaterialLibrary.CreateDynamicMaterialInstance` "/Game/M_WavyScreenFX.M_WavyScreenFX"))
  (bind _output_get_2 (set `self.WavyScreenMaterialInstance` _returnvalue_2))
  (set `PostProcessComponent.Settings` (make `PostProcessSettings` :`WeightedBlendables` (make `WeightedBlendables` (`|MakeArray` (make `WeightedBlendable` 1.0 _output_get) (make `WeightedBlendable` 1.0 _output_get_2)))) (`self.PostProcess`))
  (bind _asbp_first_person_game_mode (cast `/Game/Blueprints/BP_FirstPersonGameMode` (`GameplayStatics.GetGameMode`)))
  (add `PanaceaGameMode.OnIngredientAdded` _asbp_first_person_game_mode (delegate `OnIngredientAdded`))
  (`MaterialInstanceDynamic.SetScalarParameterValue` (`self.HallucinationMaterialInstance`) "HallucinationAmount" 0.0)
  (`MaterialInstanceDynamic.SetScalarParameterValue` (`self.WavyScreenMaterialInstance`) "WavyIntensity" 0.0))

(event `OnIngredientAdded`
  (params (IngredientName :type String))
  (bind (_direction _effect_intensity) (`Timeline|Timeline` :!via `PlayFromStart`)
    (:`Update`
      (`MaterialInstanceDynamic.SetScalarParameterValue` (`self.HallucinationMaterialInstance`) "HallucinationAmount" _effect_intensity)
      (`MaterialInstanceDynamic.SetScalarParameterValue` (`self.WavyScreenMaterialInstance`) "WavyIntensity" _effect_intensity))))

(fn `UserConstructionScript`)